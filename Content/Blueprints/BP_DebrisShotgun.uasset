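; BP_DebrisShotgun scatters debris onto surfaces by firing randomly angled line traces from its root.
; AddCubes spawns attached BP_DSMarker actors with random yaw and limited roll, then sets their trace length.
; Trace draws each marker's line trace; Build repeats them, attaching Debris to hit actors, spawning once per non-hit marker through a nested loop.
; Clear destroys the markers and empties the ignore list.
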(event `Clear`
  (bind _shotmarker (`self.ShotMarker`))
  (for (_array_element _array_index) _shotmarker :!label _label
    (`self.K2_DestroyActor` _array_element)
    (`KismetArrayLibrary.Array_Remove` _shotmarker _array_index)
    (`KismetArrayLibrary.Array_Clear` (`self.IgnoreList`)))
  (if (not (== (`KismetArrayLibrary.Array_Length` _shotmarker) 0))
    (goto _label)))

(event `AddCubes`
  (bind _shotmarker (`self.ShotMarker`))
  (bind _returnvalue (/ (`self.MaxAngle`) 2.0))
  (`KismetArrayLibrary.Array_Add` (`self.IgnoreList`) self)
  (for _ (`self.Shot#`)
    (bind _returnvalue_2 (`|SpawnActorFromClass` "/Game/Blueprints/DebrisShotgun/BP_DSMarker.BP_DSMarker_C" (`KismetMathLibrary.MakeTransform` (`SceneComponent.K2_GetComponentLocation` (`self.DefaultSceneRoot`)) (`KismetMathLibrary.MakeRotator` (+ (`KismetMathLibrary.RandomFloatInRange` (* _returnvalue -1.0) _returnvalue) 180.0) 0.0 (`KismetMathLibrary.RandomFloatInRange` -360.0 360.0))) "Undefined" "OverrideRootScale" self null))
    (`KismetArrayLibrary.Array_Add` _shotmarker _returnvalue_2)
    (`KismetArrayLibrary.Array_Add` (`self.IgnoreList`) _returnvalue_2)
    (`self.K2_AttachToActor` _returnvalue_2 self "None" "KeepWorld" "KeepWorld" "KeepWorld" true))
  (for _array_element _shotmarker
    (`/Game/Blueprints/DebrisShotgun/BP_DSMarker.Update` _array_element (`self.TraceLength`))))

(event `Trace`
  (for _array_element (`self.ShotMarker`)
    (`KismetSystemLibrary.LineTraceSingle` (`SceneComponent.K2_GetComponentLocation` (`/Game/Blueprints/DebrisShotgun/BP_DSMarker.Start` _array_element)) (`SceneComponent.K2_GetComponentLocation` (`/Game/Blueprints/DebrisShotgun/BP_DSMarker.End` _array_element)) "TraceTypeQuery1" false (`self.IgnoreList`) "ForDuration")))

(event `Build`
  (for _array_element (`self.ShotMarker`)
    (bind _outhit (`KismetSystemLibrary.LineTraceSingle` (`SceneComponent.K2_GetComponentLocation` (`/Game/Blueprints/DebrisShotgun/BP_DSMarker.Start` _array_element)) (`SceneComponent.K2_GetComponentLocation` (`/Game/Blueprints/DebrisShotgun/BP_DSMarker.End` _array_element)) "TraceTypeQuery1" false (`self.IgnoreList`) "ForDuration"))
    (for _array_element_2 (`self.ShotMarker`)
      (bind (_bblockinghit _binitialoverlap _time _distance _location _impactpoint _normal _impactnormal _physmat _hitactor) (`GameplayStatics.BreakHitResult` _outhit))
      (if (not (== _array_element_2 _hitactor))
        (bind _returnvalue (`|SpawnActorFromClass` "/Game/Blueprints/DebrisShotgun/Debris.Debris_C" (`KismetMathLibrary.Conv_VectorToTransform` _location) "Undefined" "OverrideRootScale" null null))
        (`self.K2_AttachToActor` _returnvalue _hitactor "None" "KeepWorld" "KeepWorld" "KeepWorld" true)))))

(fn `UserConstructionScript`)