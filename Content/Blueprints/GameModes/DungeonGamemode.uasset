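; Dungeon game mode that builds level contents from color-coded maps and drives the Tormentor, minimap and background music.
; Color callbacks add tiles and register player, Tormentor, eye and monster spawns, or place traps and murals wired to tile events.
; Minimap setup also spawns queued monsters per room, and player actions trace for tiles to reveal outside boss levels.
; Collecting an eye spawns the Tormentor farthest from the player; collecting all despawns enemies.
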(event `AddEmptyTile`
  (params (room :type "DungeonRoomTileBase Object Reference") (position :type "Vector2D Structure"))
  (`DungeonRoomTileBase.AddTile` room position))

(event `AddTormentorSpawn`
  (params (room :type "DungeonRoomTileBase Object Reference") (position :type "Vector2D Structure"))
  (bind _returnvalue (`DungeonRoomTileBase.AddTile` room position))
  (`self.AddTormentorLocation` _returnvalue))

(event `SpawnPlayer`
  (params (room :type "DungeonRoomTileBase Object Reference") (position :type "Vector2D Structure"))
  (bind _returnvalue (`DungeonRoomTileBase.AddTile` room position))
  (`self.SetPlayerLocation` _returnvalue))

(event `SpawnEye`
  (params (room :type "DungeonRoomTileBase Object Reference") (position :type "Vector2D Structure"))
  (`|ExecutionSequence`
    (:`then_0`
      (`DungeonRoomTileBase.AddTile` room position))
    (:`then_1`
      (`self.AddEyeLocation` room position))))

(event `SpawnMonster`
  (params (room :type "DungeonRoomTileBase Object Reference") (position :type "Vector2D Structure"))
  (`self.Enemy Spawn Logic` room position "/Game/Blueprints/C_BPExtensions/DungeonCreatureZombie.DungeonCreatureZombie_C"))

(event `TrapSpawnEvent`
  (params (room :type "DungeonRoomTileBase Object Reference") (position :type "Vector2D Structure"))
  (bind _returnvalue (`DungeonRoomTileBase.AddTile` room position))
  (add `DungeonSingleTile.TileEvent` _returnvalue (delegate `CustomEvent_Wham`))
  (bind _returnvalue_2 (`|SpawnActorFromClass` "/Game/Blueprints/TrapBaseBP.TrapBaseBP_C" (`self.GetTransform` _returnvalue) "Undefined" "OverrideRootScale" null null))
  (`self.K2_AttachToActor` _returnvalue_2 _returnvalue "None" "KeepWorld" "KeepWorld" "KeepWorld" false)
  (`/Game/Blueprints/TrapBaseBP.TrapSpawnCall` _returnvalue_2))

(event `CustomEvent_Wham`
  (params (Occupant :type "Actor Object Reference") (TriggeredTile :type "DungeonSingleTile Object Reference"))
  (for _array_element (`self.GetAttachedActors` TriggeredTile)
    (bind _astrap_base_bp (cast `/Game/Blueprints/TrapBaseBP` _array_element))
    (`/Game/Blueprints/TrapBaseBP.TrapActivate` _astrap_base_bp Occupant)))

(event `MuralEyeCheckTrigger`
  (params (Occupant :type "Actor Object Reference") (TriggeredTile :type "DungeonSingleTile Object Reference"))
  (bind _asdungeon_crawler_player (cast `DungeonCrawlerPlayer` Occupant))
  (`/Game/Blueprints/EyeCheckerBP.StepTriggerEvent` (`self.Mural`) _asdungeon_crawler_player))

(event `MuralSpawnEvent`
  (params (room :type "DungeonRoomTileBase Object Reference") (position :type "Vector2D Structure"))
  (bind _returnvalue (`DungeonRoomTileBase.AddTile` room position))
  (bind _returnvalue_2 (`|SpawnActorFromClass` "/Game/Blueprints/EyeCheckerBP.EyeCheckerBP_C" (`KismetMathLibrary.MakeTransform` (`self.K2_GetActorLocation` _returnvalue)) "Undefined" "OverrideRootScale" null null))
  (set `/Game/Blueprints/EyeCheckerBP.Associated Tile` _returnvalue _returnvalue_2)
  (set `self.Mural` _returnvalue_2)
  (add `DungeonSingleTile.TileEvent` _returnvalue (delegate `MuralEyeCheckTrigger`))
  (bind _asroom_mural (cast `/Game/Blueprints/Rooms/RoomMural` (`DungeonMacroGrid.GetRoom` (`self.DungeonMap`) (`DungeonMacroGrid.WorldToRoomPosition` (`self.K2_GetActorLocation` _returnvalue)))))
  (bind _output_get (set `/Game/Blueprints/Rooms/RoomMural.MuralChecker` (`self.Mural`) _asroom_mural))
  (bind _asdungeon_crawler_player_bp (cast `/Game/Blueprints/C_BPExtensions/DungeonCrawlerPlayerBP` (`self.ActivePlayer`)))
  (`/Game/Blueprints/C_BPExtensions/DungeonCrawlerPlayerBP.Bind All Eyes Collected To Hint` _asdungeon_crawler_player_bp _output_get))

(event `self.BindColorMapEvents`
  (`|ExecutionSequence`
    (:`then_0`
      (`self.AddColorMap` (`self.MakeRGBColor` 0) (delegate `AddEmptyTile`))
      (`self.AddColorMap` (`self.MakeRGBColor` 255) (delegate `AddTormentorSpawn`))
      (`self.AddColorMap` (`self.MakeRGBColor` 0 255) (delegate `SpawnPlayer`))
      (`self.AddColorMap` (`self.MakeRGBColor` 0 255 255) (delegate `SpawnEye`))
      (`self.AddColorMap` (`self.MakeRGBColor` 255 255) (delegate `SpawnMonster`))
      (`self.AddColorMap` (`self.MakeRGBColor` 255 0 255) (delegate `TrapSpawnEvent`))
      (`self.AddColorMap` (`self.MakeRGBColor` 0 0 255) (delegate `MuralSpawnEvent`)))
    (:`then_1`
      (bind _asdungeon_game_instance (cast `/Game/Blueprints/DungeonGameInstance` (`GameplayStatics.GetGameInstance`))
        (:`then`
          (bind _output_get (set `self.GameInstance` _asdungeon_game_instance))
          (if (not (`/Game/Blueprints/DungeonGameInstance.BGPlaying` _output_get))
            (bind _bgsfx (`/Game/Blueprints/DungeonGameInstance.BGSFX` _output_get))
            (`/Engine/EditorBlueprintResources/StandardMacros.IsValid` _bgsfx
              (:`Is Valid`
                (`AudioComponent.FadeIn` _bgsfx 2.0 1.0 0.0)))))
        (:`CastFailed`
          (`KismetSystemLibrary.PrintString` "GameInstance Cast Failed"))))))

(event `self.PlayerAction`
  (if (not (`self.bIsBossLevel?`))
    (`self.Track Minimap Update`)))

(event `Eye Collected`
  (`self.Spawn Tormentor`))

(event `AllEyesCollected`
  (bind _gameinstance (`self.GameInstance`))
  (`self.DespawnEnemies`)
  (`AudioComponent.FadeOut` (`/Game/Blueprints/DungeonGameInstance.BGSFX` _gameinstance) 5.0 0.0)
  (set `/Game/Blueprints/DungeonGameInstance.BGPlaying` false _gameinstance))

(event `self.BeginGame`
  (bind _room_to_spawn_info_dict (`self.Room To Spawn Info Dict`))
  (bind _dungeon_edge_scale (`self.Dungeon Edge Scale`))
  (bind _returnvalue (/ _dungeon_edge_scale 2.0))
  (if (not (`self.bIsBossLevel?`))
    (set `self.Dungeon Edge Scale` (`KismetMathLibrary.Conv_IntToDouble` (* (`DungeonMacroGrid.MapMaxWidth` (`self.DungeonMap`)) (`DungeonRoomTileBase.GetRoomPositionScalar`))))
    (bind _returnvalue_2 (`|SpawnActorFromClass` "/Game/Blueprints/Minimapper.Minimapper_C" (`KismetMathLibrary.MakeTransform` (0.0 0.0 0.0)) "Undefined" "OverrideRootScale" null null))
    (bind _output_get (set `self.Minimapper` _returnvalue_2))
    (bind _keys (`BlueprintMapLibrary.Map_Keys` _room_to_spawn_info_dict))
    (for _array_element _keys
      (`DungeonRoomTileBase.SpawnEnemies` _array_element (`BlueprintMapLibrary.Map_Find` _room_to_spawn_info_dict _array_element)))
    (`/Game/Blueprints/Minimapper.Init Camera` _output_get (`KismetMathLibrary.MakeVector` _returnvalue _returnvalue) _dungeon_edge_scale))
  (if (not (and (not (`KismetSystemLibrary.IsValid` (`self.ActiveTormentor`))) (> (`KismetArrayLibrary.Array_Length` (`self.tormentorSpawnLocations`)) 0)))
    (`KismetSystemLibrary.PrintString` "ERROR: No spawn locations for tormentor!" true true (struct :`R` 1.0 :`A` 1.0))))

(event `self.ReceiveTick`
  (params (DeltaSeconds :type "Float (single-precision)"))
  (`self.DoTormentorAction`))

(fn `Enemy Spawn Logic`
  (params (Room :type "DungeonRoomTileBase Object Reference") (Position :type "Vector2D Structure") (Type :type "DungeonCrawlerEnemy Class Reference"))
  (locals (Container :type "EnemySpawnDataArrayContainer Structure"))
  (`|ExecutionSequence`
    (:`then_0`
      (bind _output_get (set `local.Container` (`BlueprintMapLibrary.Map_Find` (`self.Room To Spawn Info Dict`) Room)))
      (`KismetArrayLibrary.Array_Add` (`.DataArray` (break `EnemySpawnDataArrayContainer` _output_get)) (make `EnemySpawnData` Position Type))
      (`BlueprintMapLibrary.Map_Add` (`self.Room To Spawn Info Dict`) Room (`local.Container`)))
    (:`then_1`
      (`DungeonRoomTileBase.AddTile` Room Position))))

(fn `Get Furthest Tormentor Spawn`
  (params (`Spawn Locations` :type "Array of DungeonSingleTile Object Reference"))
  (returns (`Spawn Tile` :type "DungeonSingleTile Object Reference"))
  (locals (`Longest DIst` :type "Float (double-precision)") (`Tormentor Spawn Tile` :type "DungeonSingleTile Object Reference"))
  (bind _output_get (set `local.Tormentor Spawn Tile` (`|GetArrayItem` `Spawn Locations`)))
  (set `local.Longest DIst` (`self.GetSquaredDistanceTo` (`self.ActivePlayer`) _output_get))
  (for _array_element `Spawn Locations`
    (bind _returnvalue (`self.GetSquaredDistanceTo` _array_element (`self.ActivePlayer`)))
    (if (> _returnvalue (`local.Longest DIst`))
      (set `local.Tormentor Spawn Tile` _array_element)
      (set `local.Longest DIst` _returnvalue)))
  (return (`local.Tormentor Spawn Tile`)))

(fn `Get Random Tormentor Spawn`
  (params (`Spawn Locations` :type "Array of DungeonSingleTile Object Reference"))
  (returns (`Spawn Tile` :type "DungeonSingleTile Object Reference"))
  (locals (`Int Array` :type "Array of Integer") (Tile :type "DungeonSingleTile Object Reference"))
  (bind _returnvalue (`KismetArrayLibrary.Array_Length` `Spawn Locations`))
  (bind _int_array (`local.Int Array`))
  (bind _tile (`local.Tile`))
  (`KismetArrayLibrary.Array_Resize` (`local.Int Array`) _returnvalue)
  (for _index (range (+ _returnvalue 1))
    (`KismetArrayLibrary.Array_Set` _int_array _index _index)
    (return _tile))
  (`KismetArrayLibrary.Array_Shuffle` _int_array)
  (for _array_element _int_array
    (bind _output (`|GetArrayItem` `Spawn Locations` _array_element))
    (if (> (`self.GetSquaredDistanceTo` _output (`self.ActivePlayer`)) (`KismetMathLibrary.Square` (`self.Min Tormentor Spawn Spacing`)))
      (set `local.Tile` _output)
      (break)))
  (`/Engine/EditorBlueprintResources/StandardMacros.IsValid` _tile
    (:`Is Valid`
      (return _tile))
    (:`Is Not Valid`
      (`KismetSystemLibrary.PrintString` "Tormentor Spawn ERROR: No valid spawn location found..."))))

(fn `Spawn Tormentor`
  (`/Engine/EditorBlueprintResources/StandardMacros.IsValid` (`self.ActiveTormentor`)
    (:`Is Not Valid`
      (bind _spawn_tile (`self.Get Furthest Tormentor Spawn` (`self.tormentorSpawnLocations`)))
      (bind _returnvalue (`|SpawnActorFromClass` "/Game/Blueprints/C_BPExtensions/DungeonTormentorBP.DungeonTormentorBP_C" (`self.GetTransform` _spawn_tile) "Undefined" "OverrideRootScale" null null))
      (bind _output_get (set `self.activeTormentor` _returnvalue))
      (`DungeonTileOccupant.SetTile` _output_get _spawn_tile)
      (`DungeonTormentor.SetTarget` _output_get (`DungeonRoomTileBase.GetTileRandom` (`DungeonMacroGrid.GetRoomRandom` (`self.DungeonMap`)) 3) true))))

(fn `Track Minimap Update`
  (bind _activeplayer (`self.ActivePlayer`))
  (bind _returnvalue (`self.K2_GetActorLocation` _activeplayer))
  (`/Engine/EditorBlueprintResources/StandardMacros.IsValid` (`self.Minimapper`)
    (:`Is Valid`
      (bind _outhit (`KismetSystemLibrary.LineTraceSingle` (- _returnvalue (0.0 0.0 100.0)) (+ _returnvalue (0.0 0.0 100.0)) "TraceTypeQuery1" false (`|MakeArray` _activeplayer :!type "Actor Object Reference")))
      (bind (_bblockinghit _binitialoverlap _time _distance _location _impactpoint _normal _impactnormal _physmat _hitactor) (`GameplayStatics.BreakHitResult` _outhit))
      (if (`KismetMathLibrary.ClassIsChildOf` (`GameplayStatics.GetObjectClass` _hitactor) "/Script/Damnation.DungeonRoomTileBase")
        (`/Game/Blueprints/Minimapper.Add Actor` (`self.Minimapper`) _hitactor true)))))

(fn `UserConstructionScript`)