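; Base spike trap for the dungeon crawler that animates its spikes on activation and reacts to whoever triggered it.
; A timeline drives spike height and fires a hit event: players and zombies lose health, while the Tormentor boss only plays a damage animation and rare pain sound.
; Spikes reset after a delay.
; On spawn, a line trace finds the overlapping instanced floor tile and hides it by updating that instance's transform.
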(event `TrapActivate`
  (params (TriggerActor :type "Actor Object Reference"))
  ;[1 1 1] Trigger Logic
  (`GameplayStatics.PlaySoundAtLocation` "/Game/Assets/Audio/Cues/SC_TrapTrigger.SC_TrapTrigger" (`self.K2_GetActorLocation` self) (struct) 1.0 1.0 0.0 null "/Game/Assets/Audio/Concurrency_Trap.Concurrency_Trap" self)
  (bind (_direction _spikeheight) (`Timeline|SpikeCurve` :!via `PlayFromStart`)
    (:`Update`
      (`SceneComponent.K2_SetRelativeLocation` (`self.SpikeMesh`) (`KismetMathLibrary.MakeVector` 0.0 0.0 _spikeheight) false false))
    (:`SpikeHit`
      ;[1 1 1] Per-Type Logic
      (cast `DungeonCrawlerPlayer` TriggerActor
        (:`then`
          (bind _asdungeon_crawler_player_bp (cast `/Game/Blueprints/C_BPExtensions/DungeonCrawlerPlayerBP` TriggerActor))
          (`DungeonCrawlerPlayer.AlterHealth` _asdungeon_crawler_player_bp -1)
          (`/Game/Blueprints/C_BPExtensions/DungeonCrawlerPlayerBP.PlayerDamageAnim` _asdungeon_crawler_player_bp))
        (:`CastFailed`
          (bind _asdungeon_tile_occupant (cast `DungeonTileOccupant` TriggerActor))
          (bind _returnvalue (`DungeonTileOccupant.GetType` _asdungeon_tile_occupant))
          (switch `EOccupantType` _returnvalue
            (:`Boss`
              (if (>= (`KismetMathLibrary.RandomFloatInRange` 0.0 1.0) 0.999)
                (`GameplayStatics.PlaySoundAtLocation` "/Game/Assets/Audio/Cues/SC_TormentorPain.SC_TormentorPain" (`self.K2_GetActorLocation`) (struct) 1.0 5000.0 0.0 null null null))
              (bind _asdungeon_tormentor_bp (cast `/Game/Blueprints/C_BPExtensions/DungeonTormentorBP` _asdungeon_tile_occupant))
              (`/Game/Blueprints/C_BPExtensions/DungeonTormentorBP.TormentorDamageAnim` _asdungeon_tormentor_bp))
            (:`Enemy`
              (bind _asdungeon_creature_zombie (cast `/Game/Blueprints/C_BPExtensions/DungeonCreatureZombie` TriggerActor))
              (`DungeonCrawlerEnemy.AlterHealth` _asdungeon_creature_zombie -1)))))
      (`KismetSystemLibrary.Delay` 1.0)
      (`self.TrapReset`))))

(event `TrapSpawnCall`
  (bind _returnvalue (`self.K2_GetActorLocation` self))
  ;[1 1 1] Finds and hides tile occupying same position
  (`KismetSystemLibrary.Delay` 0.2)
  (bind _outhit (`KismetSystemLibrary.LineTraceSingleForObjects` (+ _returnvalue (0.0 0.0 100.0)) (- _returnvalue (0.0 0.0 100.0)) (`|MakeArray` "ObjectTypeQuery1" "ObjectTypeQuery2" :!type "EObjectTypeQuery Enum")))
  (bind (_bblockinghit _binitialoverlap _time _distance _location _impactpoint _normal _impactnormal _physmat _hitactor _hitcomponent _hitbonename _hititem) (`GameplayStatics.BreakHitResult` _outhit))
  (bind _asinstanced_static_mesh_component (cast `InstancedStaticMeshComponent` _hitcomponent))
  (`InstancedStaticMeshComponent.UpdateInstanceTransform` _asinstanced_static_mesh_component _hititem (`KismetMathLibrary.MakeTransform` (+ (.location (`InstancedStaticMeshComponent.GetInstanceTransform` _asinstanced_static_mesh_component _hititem false)) (0.0 0.0 4500.0)) (.rotation (`InstancedStaticMeshComponent.GetInstanceTransform` _asinstanced_static_mesh_component _hititem false)) (.scale (`InstancedStaticMeshComponent.GetInstanceTransform` _asinstanced_static_mesh_component _hititem false))) false true true)
  (`PrimitiveComponent.SetCastShadow` _asinstanced_static_mesh_component false)
  (`self.TrapReset`))

(event `TrapReset`
  ;[1 1 1] Reset Logic
  (`SceneComponent.K2_SetRelativeLocation` (`self.SpikeMesh`) (`self.DefaultPos`) false false))

(fn `UserConstructionScript`)