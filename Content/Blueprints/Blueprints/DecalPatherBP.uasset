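; DecalPatherBP scatters decals along a path between a start and an end on a MacroGrid.
; MakeDecalPath gets the path actors from the grid's GeneratePath and walks them with a countdown drawn randomly between minimum and maximum spawn intervals.
; When the countdown hits zero, it spawns a downward-projected decal at that actor's slightly offset location with random yaw, then rerolls the interval for irregular spacing.
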(fn `Make Decal Path`
  (params (`Macro Grid` :type "DungeonMacroGrid Object Reference") (Start :type "DungeonSingleTile Object Reference") (End :type "DungeonSingleTile Object Reference"))
  (bind _spawn_current (`self.Spawn Current`))
  (bind _returnvalue (`DungeonMacroGrid.GeneratePath` `Macro Grid` Start End 1 true false))
  (set `self.Spawn Current` (`KismetMathLibrary.RandomIntegerInRange` (`self.Spawn Interval Minimum`) (`self.Spawn Interval Maximum`)))
  (for _array_element _returnvalue
    (`|ExecutionSequence`
      (:`then_0`
        (if (== _spawn_current 0)
          (`GameplayStatics.SpawnDecalAtLocation` (`self.Decal Material`) (10.0 100.0 100.0) (+ (`self.K2_GetActorLocation` _array_element) (10.0 10.0 0.0)) (`KismetMathLibrary.MakeRotator` 0.0 90.0 (`KismetMathLibrary.RandomFloatInRange` 0.0 360.0)))
          (set `self.Spawn Current` (`KismetMathLibrary.RandomIntegerInRange` (`self.Spawn Interval Minimum`) (`self.Spawn Interval Maximum`)))))
      (:`then_1`
        (`/Engine/EditorBlueprintResources/StandardMacros.DecrementInt` _spawn_current))))
  (return))

(fn `UserConstructionScript`)