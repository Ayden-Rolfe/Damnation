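; EyeCheckerBP displays the collected eye count and fires an all-eyes-collected dispatch once six are reached.
; The construction script caches hand-placed VisibleEyes instance transforms, then removes the instances.
; StepTriggerEvent reads the triggering actor's eye count and re-adds eyes at those transforms at half scale, dispatching only once.
; On BeginPlay, line traces at stored under-tile positions remove any instanced-mesh tiles they hit, clearing overlaps.
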(event `self.ReceiveBeginPlay`
  (`self.SpawnEvent`))

(event `TransformsReset`)

(event `ForceSpawn`
  (for _array_element (`self.TransformEyeArray`)
    (`InstancedStaticMeshComponent.AddInstance` (`self.Visible Eyes`) _array_element)))

(event `Clear`
  (`InstancedStaticMeshComponent.ClearInstances` (`self.Visible Eyes`)))

(event `DEBUG Trigger Escape`
  (`self.AllEyesCollectedDispatch` :!label _label)
  (set `self.Dispatch Called` true))

(event `StepTriggerEvent`
  (params (TriggerActor :type "DungeonCrawlerPlayer Object Reference"))
  (bind _returnvalue (`DungeonCrawlerPlayer.GetEyeCount` TriggerActor))
  (`self.TransformsReset`)
  (for _index (range (`self.EyesAddedTotal`) _returnvalue)
    (`InstancedStaticMeshComponent.AddInstance` (`self.Visible Eyes`) (`KismetMathLibrary.MakeTransform` (.location (`|GetArrayItem` (`self.TransformEyeArray`) _index)) (.rotation (`|GetArrayItem` (`self.TransformEyeArray`) _index)) (0.5 0.5 0.5)))
    (bind _output_get (set `self.EyesAddedTotal` _returnvalue))
    (if (and (>= _output_get 6) (not (`self.Dispatch Called`)))
      (goto _label))))

(event `SpawnEvent`
  ;[1 1 1] Finds and deletes tile occupying same position
  (for _array_element (`self.TileUnderPosArray`)
    (bind _returnvalue (+ _array_element (`SceneComponent.K2_GetComponentLocation` (`self.TilesUnder`))))
    (bind _outhit (`KismetSystemLibrary.LineTraceSingleForObjects` (+ _returnvalue (0.0 0.0 50.0)) (- _returnvalue (0.0 0.0 50.0)) (`|MakeArray` "ObjectTypeQuery2" "ObjectTypeQuery1" :!type "EObjectTypeQuery Enum")))
    (bind (_bblockinghit _binitialoverlap _time _distance _location _impactpoint _normal _impactnormal _physmat _hitactor _hitcomponent _hitbonename _hititem) (`GameplayStatics.BreakHitResult` _outhit))
    (bind _asinstanced_static_mesh_component (cast `InstancedStaticMeshComponent` _hitcomponent))
    (`InstancedStaticMeshComponent.RemoveInstance` _asinstanced_static_mesh_component _hititem)))

(fn `UserConstructionScript`
  (locals (Count :type Integer :default 0))
  (bind _visible_eyes (`self.Visible Eyes`))
  (bind _transformeyearray (`self.TransformEyeArray`))
  (bind _returnvalue (`InstancedStaticMeshComponent.GetInstanceCount` _visible_eyes))
  (set `local.Count` _returnvalue)
  (`KismetArrayLibrary.Array_Clear` _transformeyearray)
  (`KismetArrayLibrary.Array_Resize` _transformeyearray _returnvalue)
  (for _index (range (+ (`local.Count`) 1))
    (`KismetArrayLibrary.Array_Set` (`self.TransformEyeArray`) _index (`InstancedStaticMeshComponent.GetInstanceTransform` _visible_eyes _index false)))
  (bind _arrayindex (`/Engine/EditorBlueprintResources/StandardMacros.ReverseForEachLoop` (`self.TransformEyeArray`))
    (:`LoopBody`
      (`InstancedStaticMeshComponent.RemoveInstance` _visible_eyes _arrayindex))))