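; Minimapper actor that renders a top-down minimap image through a SceneCaptureComponent2D.
; InitCamera places the capture 5000 units above a given center, pointing straight down, with its ortho width set to the given size.
; AddActor adds actors uniquely to the show-only list and optionally recaptures.
; UpdateScene captures on demand, and Tick does no work.
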(event `Init Camera`
  (params (Center :type "Vector Structure") (Size :type "Float (double-precision)"))
  (bind _scenecapturecomponent2d (`self.SceneCaptureComponent2D`))
  (set `SceneCaptureComponent2D.OrthoWidth` Size _scenecapturecomponent2d)
  (`SceneComponent.K2_SetWorldTransform` _scenecapturecomponent2d (`KismetMathLibrary.MakeTransform` (+ Center (0.0 0.0 5000.0)) (`KismetMathLibrary.MakeRotator` 0.0 -90.0)) false true))

(event `Add Actor`
  (params (Actor :type "Actor Object Reference") (`Update Image?` :type Boolean))
  (`KismetArrayLibrary.Array_AddUnique` (`SceneCaptureComponent.ShowOnlyActors` (`self.SceneCaptureComponent2D`)) Actor)
  (if `Update Image?`
    (`SceneCaptureComponent2D.CaptureScene` (`self.SceneCaptureComponent2D`))))

(event `Update Scene`
  (`SceneCaptureComponent2D.CaptureScene` (`self.SceneCaptureComponent2D`)))

(fn `UserConstructionScript`)