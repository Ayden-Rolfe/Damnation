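; Procedural hallway actor that builds a floor and two side walls from HallLength and HallWidth in its Construction Script.
; FloorTiles gets a grid of instances on 100-unit spacing, each with a random quarter-turn yaw for variation.
; LeftWall and RightWall each get one instance per length step, with RightWall offset according to the width.
; The event graph has no active logic.
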(fn `UserConstructionScript`
  (`SceneComponent.K2_SetRelativeLocation` (`self.Right Wall`) (`KismetMathLibrary.MakeVector` 50.0 (+ (* (- (`self.Hall Width`) 1) 100.0) 50.0)) false false)
  (for _index (range (`self.Hall Length`))
    (for _index_2 (range (`self.Hall Width`))
      (`InstancedStaticMeshComponent.AddInstance` (`self.Floor Tiles`) (`KismetMathLibrary.MakeTransform` (+ (* (`KismetMathLibrary.MakeVector` (`KismetMathLibrary.Conv_IntToDouble` _index) (`KismetMathLibrary.Conv_IntToDouble` _index_2)) 100.0) (50.0 50.0 0.0)) (`KismetMathLibrary.MakeRotator` 0.0 0.0 (* (`KismetMathLibrary.RandomIntegerInRange` 0 3) 90.0)))))
    (bind _returnvalue (* _index 100.0))
    (`InstancedStaticMeshComponent.AddInstance` (`self.Left Wall`) (`KismetMathLibrary.MakeTransform` (`KismetMathLibrary.MakeVector` 0.0 (* _returnvalue -1.0))))
    (`InstancedStaticMeshComponent.AddInstance` (`self.Right Wall`) (`KismetMathLibrary.MakeTransform` (`KismetMathLibrary.MakeVector` 0.0 _returnvalue)))))