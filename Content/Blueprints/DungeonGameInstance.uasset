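; Game instance for a dungeon game that owns audio options and sounds that persist across level transitions.
; On Init, after a short delay, it pushes the master sound mix, loads or creates SaveOptions, applies saved volumes and starts dungeon ambience.
; SetVolume applies clamped Master, SFX or Ambience levels as sound class overrides and passes them to SaveOptions.
; It also creates a persistent 2D UI sound, replayed through PlayUISound.
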(event `self.ReceiveInit`
  (bind (_mastervolume _sfxvolume _ambiencevolume) (break `/Game/Blueprints/Struct_SoundOptions` (`/Game/Blueprints/SaveOptions.SoundOptions` (`self.SaveOptions`))))
  (`KismetSystemLibrary.Delay` 0.2)
  (`GameplayStatics.SetBaseSoundMix` "/Game/Assets/Audio/SoundMix_Master.SoundMix_Master")
  (`GameplayStatics.PushSoundMixModifier` "/Game/Assets/Audio/SoundMix_Master.SoundMix_Master")
  (`/Engine/EditorBlueprintResources/StandardMacros.IsValid` (`self.SaveOptions`)
    (:`Is Valid`
      _)
    (:`Is Not Valid`
      (`self.LoadOptions`)))
  (`|ExecutionSequence`
    (:`then_0`
      (`self.SetVolume` "NewEnumerator0" _mastervolume))
    (:`then_1`
      (`self.SetVolume` "NewEnumerator1" _sfxvolume))
    (:`then_2`
      (`self.SetVolume` "NewEnumerator2" _ambiencevolume))
    (:`then_3`
      (`self.DungeonAmbience`)
      (`self.CreateUISound`))))

(event `PlayUISound`
  (`AudioComponent.Play` (`self.UISound`) 0.0))

(fn `CreateUISound`
  (bind _returnvalue (`GameplayStatics.CreateSound2D` "/Game/Assets/Audio/Cues/SC_UISound.SC_UISound" 1.0 1.0 0.0 null true false))
  (set `self.UISound` _returnvalue))

(fn `DungeonAmbience`
  (bind _returnvalue (`GameplayStatics.CreateSound2D` "/Game/Assets/Audio/Cues/SC_DungeonAmbience.SC_DungeonAmbience" 1.0 1.0 0.0 null true false))
  (bind _output_get (set `self.BGSFX` _returnvalue))
  (`AudioComponent.Play` _output_get 0.0)
  (set `self.BGPlaying` true)
  (`KismetSystemLibrary.PrintString` "Ambience Triggered"))

(fn `LoadOptions`
  (returns (Options :type "/Game/Blueprints/SaveOptions Object Reference"))
  (bind _returnvalue (`GameplayStatics.DoesSaveGameExist` (`self.SaveOptionsName`)))
  (if _returnvalue
    (bind _returnvalue_2 (`GameplayStatics.LoadGameFromSlot` (`self.SaveOptionsName`) :!label _label))
    (bind _assave_options (cast `/Game/Blueprints/SaveOptions` _returnvalue_2))
    (bind _output_get (set `self.SaveOptions` _assave_options))
    (else
      (`/Engine/EditorBlueprintResources/StandardMacros.IsValid` (`self.SaveOptions`)
        (:`Is Valid`
          (goto _label))
        (:`Is Not Valid`
          (bind _returnvalue_3 (`GameplayStatics.CreateSaveGameObject` "/Game/Blueprints/SaveOptions.SaveOptions_C"))
          (set `self.SaveOptions` _returnvalue_3)))))
  (return _output_get))

(fn `SetVolume`
  (params (ESoundChannel :type "/Game/Blueprints/SoundChannelEnum Enum" :default "NewEnumerator0") (Value :type "Float (double-precision)"))
  (bind _returnvalue (`KismetMathLibrary.FClamp` Value))
  (bind _saveoptions (`self.SaveOptions`))
  (bind _saveoptions_2 (`self.SaveOptions`))
  (bind _saveoptions_3 (`self.SaveOptions`))
  (`/Engine/EditorBlueprintResources/StandardMacros.IsValid` (`self.SaveOptions`)
    (:`Is Valid`
      _)
    (:`Is Not Valid`
      (`self.LoadOptions`)))
  (switch `/Game/Blueprints/SoundChannelEnum` ESoundChannel
    (:`NewEnumerator0`
      (`GameplayStatics.SetSoundMixClassOverride` "/Game/Assets/Audio/SoundMix_Master.SoundMix_Master" "/Game/Assets/Audio/SClass_Master.SClass_Master" _returnvalue)
      (bind _structout (setmembers `/Game/Blueprints/Struct_SoundOptions` :`StructRef` (`/Game/Blueprints/SaveOptions.SoundOptions` _saveoptions_2) :`MasterVolume` _returnvalue))
      (`/Game/Blueprints/SaveOptions.Set Options` _saveoptions_2 _structout))
    (:`NewEnumerator1`
      (`GameplayStatics.SetSoundMixClassOverride` "/Game/Assets/Audio/SoundMix_Master.SoundMix_Master" "/Game/Assets/Audio/SClass_SFX.SClass_SFX" _returnvalue)
      (bind _structout_2 (setmembers `/Game/Blueprints/Struct_SoundOptions` :`StructRef` (`/Game/Blueprints/SaveOptions.SoundOptions` _saveoptions_3) :`SFXVolume` _returnvalue))
      (`/Game/Blueprints/SaveOptions.Set Options` _saveoptions_3 _structout_2))
    (:`NewEnumerator2`
      (`GameplayStatics.SetSoundMixClassOverride` "/Game/Assets/Audio/SoundMix_Master.SoundMix_Master" "/Game/Assets/Audio/SClass_Ambience.SClass_Ambience" _returnvalue)
      (bind _structout_3 (setmembers `/Game/Blueprints/Struct_SoundOptions` :`StructRef` (`/Game/Blueprints/SaveOptions.SoundOptions` _saveoptions) :`AmbienceVolume` _returnvalue))
      (`/Game/Blueprints/SaveOptions.Set Options` _saveoptions _structout_3))))