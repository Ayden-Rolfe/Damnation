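; Dasher enemy for the tile-based dungeon that charges in straight lines, damaging players or fellow enemies it runs into.
; On MoveAction, DasherLogic either picks a random connected cardinal direction or advances one tile, with a reticle telegraphing the next tile.
; Collisions and walls end the charge, and ActionTime paces most steps.
; The player line-of-sight helper is not used by the charge logic, and the hurt color fade is disconnected.
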(event `self.ReceiveBeginPlay`)

(event `self.ReceiveTick`
  (params (DeltaSeconds :type "Float (single-precision)")))

(event `self.ReceiveMoveAction`
  (`self.Dasher Logic`))

(event `self.ReceiveTakeDamage`
  (set `self.Hurt Effect Value` 1.0))

(event `self.ReceiveOnDeath`
  (cast `/Game/Blueprints/DungeonGamemode` (`self.Gamemode`)))

(fn `Dasher Logic`
  (locals (`Valid Directions` :type "Array of ECardinal Enum"))
  (bind _next (`self.Get Next Tile`))
  (bind _next_2 (`self.Get Next Tile`))
  (bind _valid_directions (`local.Valid Directions`))
  (bind _reticle (`self.Reticle`))
  (bind _occupyingactor (`DungeonSingleTile.OccupyingActor` _next_2))
  (if (> (`self.Health`) 0)
    (if (`self.Direction Picked`)
      (`/Engine/EditorBlueprintResources/StandardMacros.IsValid` _next_2
        (:`Is Valid`
          (`/Engine/EditorBlueprintResources/StandardMacros.IsValid` _occupyingactor
            (:`Is Valid`
              ;[1 0 0] Ran into something, stop & deal damage (if necessary)
              (bind _asdungeon_crawler_player (cast `DungeonCrawlerPlayer` _occupyingactor)
                (:`then`
                  (`DungeonCrawlerPlayer.AlterHealth` _asdungeon_crawler_player -1))
                (:`CastFailed`
                  (bind _asdungeon_tile_occupant (cast `DungeonTileOccupant` _occupyingactor))
                  (bind _returnvalue (`self.GetType` _asdungeon_tile_occupant))
                  (switch `EOccupantType` _returnvalue
                    (:`Boss`
                      _)
                    (:`Enemy`
                      (`self.AlterHealth` (cast `DungeonCrawlerEnemy` _asdungeon_tile_occupant :!pure true) -1))
                    (:`Eye`
                      _))))
              (set `self.Direction Picked` false)
              (`SceneComponent.SetVisibility` (`self.Reticle`) false true))
            (:`Is Not Valid`
              ;[1 0.196 0] Continue charge
              ; Set position of both this & reticle, accordingly
              (`self.SetTile` _next)
              (`/Engine/EditorBlueprintResources/StandardMacros.IsValid` _next
                (:`Is Valid`
                  (`SceneComponent.K2_SetWorldLocation` (`self.Reticle`) (+ (`self.K2_GetActorLocation` _next) (0.0 0.0 10.0)) false true))
                (:`Is Not Valid`
                  (`SceneComponent.SetVisibility` (`self.Reticle`) false true)))))
          (set `self.TimeUntilActionPermitted` (`self.ActionTime`) :!label _label))
        (:`Is Not Valid`
          (set `self.Direction Picked` false) ; Ran into a wall, pick a new direction
        ))
      (else
        ;[0 1 0] Pick random valid direction for next charge
        (`KismetArrayLibrary.Array_Clear` _valid_directions)
        (for _index (range 4)
          (`/Engine/EditorBlueprintResources/StandardMacros.IsValid` (`|GetArrayItem` (`DungeonSingleTile.CardinalConnections` (`self.CurrentTile`)) _index)
            (:`Is Valid`
              (`KismetArrayLibrary.Array_Add` (`local.Valid Directions`) (cast `ECardinal` (`KismetMathLibrary.Conv_IntToByte` _index))))))
        (set `self.TargetDirection` (`|GetArrayItem` _valid_directions (`KismetMathLibrary.RandomIntegerInRange` 0 (- (`KismetArrayLibrary.Array_Length` _valid_directions) 1))))
        (set `self.Direction Picked` true)
        (`SceneComponent.SetVisibility` _reticle true true)
        (`SceneComponent.K2_SetWorldLocation` _reticle (+ (`self.K2_GetActorLocation` (`self.Get Next Tile`)) (0.0 0.0 10.0)) false true)
        (goto _label)))))

(fn `UserConstructionScript`
  (bind _staticmesh (`self.StaticMesh`))
  (`SceneComponent.SetVisibility` (`self.Reticle`) false true)
  (`PrimitiveComponent.SetMaterial` _staticmesh 0 "/Game/Assets/Materials/MatI_EnemyTest.MatI_EnemyTest")
  (`MeshComponent.SetScalarParameterValueOnMaterials` _staticmesh "Alpha" 0.0))