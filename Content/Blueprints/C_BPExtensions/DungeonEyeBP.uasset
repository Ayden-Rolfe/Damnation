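; DungeonEyeBP is a collectible eye in a tile-based dungeon crawler, counted on the player and reported to the game mode.
; CollectEye fires a radial impulse, frees its tile for pathing, removes the eye visuals, plays a sound and triggers the player's heal animations and HUD count.
; An IsCollected flag guards against repeat pickup, and CollectEye returns whether this call collected it.
; OnCollect is a simpler pickup event without the tile, impulse or game mode updates.
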(event `self.OnCollect`
  (if (not (`self.IsCollected`))
    (`ActorComponent.K2_DestroyComponent` (`self.Eye`))
    (`ActorComponent.Deactivate` (`self.P_EyePart`))
    (`GameplayStatics.PlaySound2D` "/Game/Assets/Audio/Cues/SC_EyePickup.SC_EyePickup" 1.0 1.0 0.0 null null)
    (bind _asdungeon_crawler_player_bp (cast `/Game/Blueprints/C_BPExtensions/DungeonCrawlerPlayerBP` (`GameplayStatics.GetPlayerPawn` 0)))
    (`DungeonCrawlerPlayer.AddEye` _asdungeon_crawler_player_bp)
    (set `self.IsCollected` true)
    (bind _hudref (`/Game/Blueprints/C_BPExtensions/DungeonCrawlerPlayerBP.HUDRef` _asdungeon_crawler_player_bp))
    (`/Game/Blueprints/UI/GameHUD.Full Heal Animation` _hudref 0.0)
    (`/Game/Blueprints/UI/GameHUD.Eye Collected` _hudref (`DungeonCrawlerPlayer.GetEyeCount` _asdungeon_crawler_player_bp))
    (`KismetSystemLibrary.PrintString` "Eye collected!")))

(fn `Collect Eye`
  (returns (`Collection Valid?` :type Boolean))
  (locals (`Was Collected` :type Boolean))
  (bind _currenttile (`self.CurrentTile`))
  (bind _output_get (set `local.Was Collected` (`self.IsCollected`)))
  (if (not _output_get)
    (`RadialForceComponent.FireImpulse` (`self.RadialForce`))
    (set `DungeonSingleTile.OccupyingActor` null _currenttile)
    (`DungeonSingleTile.PermitPathing` _currenttile true)
    (`ActorComponent.K2_DestroyComponent` (`self.Eye`))
    (`ActorComponent.Deactivate` (`self.P_EyePart`))
    (`GameplayStatics.PlaySound2D` "/Game/Assets/Audio/Cues/SC_EyePickup.SC_EyePickup" 1.0 1.0 0.0 null null)
    (bind _asdungeon_crawler_player_bp (cast `/Game/Blueprints/C_BPExtensions/DungeonCrawlerPlayerBP` (`GameplayStatics.GetPlayerPawn` 0)))
    (`DungeonCrawlerPlayer.AddEye` _asdungeon_crawler_player_bp)
    (set `self.IsCollected` true)
    (bind _hudref (`/Game/Blueprints/C_BPExtensions/DungeonCrawlerPlayerBP.HUDRef` _asdungeon_crawler_player_bp))
    (`/Game/Blueprints/UI/GameHUD.Full Heal Animation` _hudref (`KismetMathLibrary.Conv_IntToDouble` (`DungeonCrawlerPlayer.GetHealth` _asdungeon_crawler_player_bp)))
    (`/Game/Blueprints/C_BPExtensions/DungeonCrawlerPlayerBP.PlayerHealAnim` _asdungeon_crawler_player_bp)
    (`/Game/Blueprints/UI/GameHUD.Eye Collected` _hudref (`DungeonCrawlerPlayer.GetEyeCount` _asdungeon_crawler_player_bp))
    (`KismetSystemLibrary.PrintString` "Eye collected!" false)
    (bind _asdungeon_gamemode (cast `/Game/Blueprints/DungeonGamemode` (`self.Gamemode`)))
    (`/Game/Blueprints/DungeonGamemode.Eye Collected` _asdungeon_gamemode))
  (return (not (`local.Was Collected`))))

(fn `UserConstructionScript`)