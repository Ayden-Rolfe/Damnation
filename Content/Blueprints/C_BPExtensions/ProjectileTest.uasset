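; Test projectile that steps across a dungeon-crawler MacroGrid and damages the player.
; Spawn stores the grid and direction, and each ProjectileAction calls MoveAction to teleport to the next position.
; On a valid tile, DamagePlayer either takes one health from an occupying player or snaps the projectile to the empty tile.
; Off the grid, it clears CurrentTile and returns the line-trace result.
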(event `Spawn`
  (params (Direction :type "Vector2D Structure") (MacroGrid :type "DungeonMacroGrid Object Reference (by ref)") (StartTile :type "DungeonSingleTile Object Reference"))
  (set `self.Macro Grid` MacroGrid)
  (set `self.DeltaPosition` Direction))

(fn `DamagePlayer`
  (params (TargetTile :type "DungeonSingleTile Object Reference"))
  (returns (ToDestroy :type Boolean))
  (bind _occupyingactor (`DungeonSingleTile.OccupyingActor` TargetTile))
  (`/Engine/EditorBlueprintResources/StandardMacros.IsValid` _occupyingactor
    (:`Is Valid`
      (bind _asdungeon_crawler_player (cast `DungeonCrawlerPlayer` _occupyingactor))
      (`DungeonCrawlerPlayer.AlterHealth` _asdungeon_crawler_player -1)
      (return true))
    (:`Is Not Valid`
      (bind _output_get (set `self.CurrentTile` TargetTile))
      (`self.K2_SetActorLocation` (`self.K2_GetActorLocation` _output_get))
      (return false))))

(fn `MoveAction`
  (returns (ToDelete :type Boolean))
  (locals (NextPosition :type "Vector Structure"))
  (bind _traceoffset (`self.TraceOffset`))
  (bind _nextposition (`local.NextPosition`))
  (bind _returnvalue (`DungeonMacroGrid.GetTileAtWorldPosition` (`self.Macro Grid`) _nextposition))
  (bind _output_get (set `local.NextPosition` (`self.Get Next Position`)))
  (bind (_outhit _returnvalue_2) (`KismetSystemLibrary.LineTraceSingle` (+ _traceoffset (`self.K2_GetActorLocation`)) (+ _output_get _traceoffset) "TraceTypeQuery4"))
  (`self.K2_SetActorLocation` _nextposition)
  (`/Engine/EditorBlueprintResources/StandardMacros.IsValid` _returnvalue
    (:`Is Valid`
      (bind _todestroy (`self.DamagePlayer` _returnvalue))
      (return _todestroy))
    (:`Is Not Valid`
      (set `self.CurrentTile` null)
      (return _returnvalue_2))))

(fn `ProjectileAction`
  (returns (ReturnValue :type Boolean))
  (bind _todelete (`self.MoveAction`))
  (return _todelete))

(fn `UserConstructionScript`)