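; Snake enemy for a tile-based dungeon crawler that attacks along diagonals.
; On its move action, it runs a sight check and requires both a hit on the player and exact diagonal tile alignment with them.
; It then fires projectiles in all four diagonal directions, registering each with the game mode and initializing it on the dungeon map.
; The move action contains no movement logic.
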(event EventMoveAction
  (CallFunction|MoveActionFunc))

(fn ConstructionScript)

(fn MoveActionFunc
  (bind _returnvalue (Transformation|GetActorLocation))
  (bind _gamemode (Variables|Default|Getgamemode))
  (bind _gamemode_2 (Variables|Default|Getgamemode))
  (bind _returnvalue_2 (Class|DungeonMacroGrid|WorldtoTilePosition _returnvalue))
  (bind _activeplayer (Variables|/Script/Damnation.DamnationGameModeBase|GetactivePlayer _gamemode))
  (bind _returnvalue_3 (Transformation|GetActorLocation _activeplayer))
  (bind (_x _y) (Math|Vector2D|BreakVector2D _returnvalue_2))
  (bind _returnvalue_4 (Class|DungeonMacroGrid|WorldtoTilePosition _returnvalue_3))
  (bind (_x_2 _y_2) (Math|Vector2D|BreakVector2D _returnvalue_4))
  (|CanSeePlayer
    (:true
      (if (|((abs((x1-x2)))==(abs((y1-y2)))) _x_2 _x _y_2 _y) ; Player is diagonally aligned
        (for _index (range 0 3)
          (bind _returnvalue_5 (Game|SpawnActorfromClass "/Game/Blueprints/C_BPExtensions/ProjectileTest.ProjectileTest_C" (Math|Transform|MakeTransform (Transformation|GetActorLocation) (Math|Rotator|MakeRotator 0.0 0.0 (+ (* _index 9e+01) 45.0))) "Undefined" 0 0)) ; FIRE
          (Utilities|Array|Add (Variables|/Script/Damnation.DamnationGameModeBase|GetactiveProjectiles _gamemode_2) _returnvalue_5)
          (Default|Spawn _returnvalue_5 (Utilities|Array|Get(acopy) (Utilities|Array|MakeArray "(X=1.000000,Y=1.000000)" "(X=-1.000000,Y=1.000000)" "(X=-1.000000,Y=-1.000000)" "(X=1.000000,Y=-1.000000)") _index) (Variables|/Script/Damnation.DamnationGameModeBase|GetDungeonMap _gamemode_2)))))))