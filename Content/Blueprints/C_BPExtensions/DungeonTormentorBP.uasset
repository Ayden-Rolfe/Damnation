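; Tormentor enemy for a tile-based dungeon crawler, with telegraphed slam and swipe attacks.
; The first attack call stores facing-based tiles, shows the area and glows red; the next damages the player or enemies on those tiles, then cleans up.
; Material timelines flash hurt or block feedback, and spotting or failing to reach the player plays a roar.
; Physics simulates bones below a target bone during life and the whole mesh on death.
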(event `self.ReceiveBeginPlay`
  (bind _tormentor_mesh (`self.Tormentor Mesh`))
  (bind _targetbone (`self.TargetBone`))
  (`AudioComponent.Play` (`self.TormentorBreathing`) 0.0)
  (`KismetSystemLibrary.Delay` 0.2)
  (`SkeletalMeshComponent.SetAllBodiesBelowSimulatePhysics` _tormentor_mesh _targetbone true false)
  (`SkeletalMeshComponent.SetAllBodiesBelowPhysicsBlendWeight` _tormentor_mesh _targetbone 1.0 false false)
  (`PrimitiveComponent.SetMassScale` _tormentor_mesh _targetbone 2.0))

(event `self.ReceiveMoveAction`)

(event `self.ReceiveOnMove`
  (params (oldPos :type "Transform Structure") (newPos :type "Transform Structure")))

(event `self.AttackSlam`
  (if (not (`self.bIsAttackPrepared`))
    (`self.Attack Preparation` (`self.GetSlamAttackTiles` (`self.Facing`))) ; Preparing slam...
    (`SceneComponent.SetVisibility` (`self.Slam Area`) true true)
    (`self.OnTormentorAttackAction` "SLAM")
    (else
      (`self.Attack Selected Tiles`) ; Performing slam
      (`self.Attack Cleanup`))))

(event `TormentorDamageAnim`
  (bind _tormentor_mesh (`self.Tormentor Mesh`))
  (if (`self.bIsVulnerable`)
    (`MeshComponent.SetVectorParameterValueOnMaterials` _tormentor_mesh "HighGlowColour" (25.0 10.0 2.0))
    (bind (_direction _alpha) (`Timeline|TormentorHurtTimeline` :!via `PlayFromStart`)
      (:`Update`
        (`MeshComponent.SetScalarParameterValueOnMaterials` _tormentor_mesh "Alpha" _alpha))
      (:`Finished`
        (if (`self.bIsAttackPrepared`) :!label _label
          (`MeshComponent.SetVectorParameterValueOnMaterials` _tormentor_mesh "HighGlowColour" (10.0 0.0 0.0))
          (`MeshComponent.SetScalarParameterValueOnMaterials` _tormentor_mesh "Alpha" 1.0))))
    (else
      (`MeshComponent.SetVectorParameterValueOnMaterials` _tormentor_mesh "HighGlowColour" (10.0 0.0 0.0))
      (bind (_direction_2 _alpha_2) (`Timeline|TormentorBlockTimeline` :!via `PlayFromStart`)
        (:`Update`
          (`MeshComponent.SetScalarParameterValueOnMaterials` _tormentor_mesh "Alpha" _alpha_2))
        (:`Finished`
          (goto _label))))))

(event `self.AttackSwipe`
  (if (not (`self.bIsAttackPrepared`))
    (`self.Attack Preparation` (`self.GetSwipeAttackTiles` (`self.Facing`)))
    (`SceneComponent.SetVisibility` (`self.Swipe Area`) true true)
    (`self.OnTormentorAttackAction` "SWIPE")
    (else
      (`self.Attack Selected Tiles`)
      (`self.Attack Cleanup`))))

(event `self.ReceiveOnCannotReachTarget`
  (`|PlayMontage` (`self.Tormentor Mesh`) (`self.Roar Animation`) :!label _label_2))

(event `self.ReceiveOnSpotPlayer`
  (goto _label_2))

(event `self.ReceiveOnDeath`
  ;[1 1 1] Tormentor Death Functionality
  (`PrimitiveComponent.SetSimulatePhysics` (`self.Tormentor Mesh`) true)
  (`self.Attack Cleanup`))

(fn `Attack Cleanup`
  (set `self.bIsAttacking` false)
  (set `self.bIsAttackPrepared` false)
  (`KismetArrayLibrary.Array_Clear` (`self.Attack Tiles`))
  (`MeshComponent.SetScalarParameterValueOnMaterials` (`self.Tormentor Mesh`) "Alpha" 0.0)
  (`SceneComponent.SetVisibility` (`self.Slam Area`) false true)
  (`SceneComponent.SetVisibility` (`self.Swipe Area`) false true))

(fn `Attack Preparation`
  (params (Tiles :type "Array of DungeonSingleTile Object Reference"))
  (bind _tormentor_mesh (`self.Tormentor Mesh`))
  (for _array_element Tiles
    (`/Engine/EditorBlueprintResources/StandardMacros.IsValid` _array_element
      (:`Is Valid`
        (`KismetArrayLibrary.Array_Add` (`self.Attack Tiles`) _array_element))))
  (set `self.bIsAttackPrepared` true)
  (`MeshComponent.SetScalarParameterValueOnMaterials` _tormentor_mesh "Alpha" 1.0)
  (`MeshComponent.SetVectorParameterValueOnMaterials` _tormentor_mesh "HighGlowColour" (10.0 0.0 0.0)))

(fn `Attack Selected Tiles`
  (for _array_element (`self.Attack Tiles`)
    (bind _occupyingactor (`DungeonSingleTile.OccupyingActor` _array_element))
    (`/Engine/EditorBlueprintResources/StandardMacros.IsValid` _occupyingactor
      (:`Is Valid`
        (bind _asdungeon_crawler_player_bp (cast `/Game/Blueprints/C_BPExtensions/DungeonCrawlerPlayerBP` _occupyingactor)
          (:`then`
            (`DungeonCrawlerPlayer.AlterHealth` _asdungeon_crawler_player_bp -1)
            (`/Game/Blueprints/C_BPExtensions/DungeonCrawlerPlayerBP.PlayerDamageAnim` _asdungeon_crawler_player_bp))
          (:`CastFailed`
            (bind _asdungeon_tile_occupant (cast `DungeonTileOccupant` _occupyingactor :!pure true))
            (bind _returnvalue (`self.GetType` _asdungeon_tile_occupant))
            (switch `EOccupantType` _returnvalue
              (:`Enemy`
                (`DungeonCrawlerEnemy.AlterHealth` (cast `DungeonCrawlerEnemy` _asdungeon_tile_occupant :!pure true) -2))))))))
  (`DamnationGameModeBase.CleanupDeadEnemies` (`self.Gamemode`))
  (return))

(fn `AttackFunc`
  (params (Object :type "Actor Object Reference"))
  (bind _asdungeon_crawler_player (cast `DungeonCrawlerPlayer` Object)
    (:`then`
      (`DungeonCrawlerPlayer.AlterHealth` _asdungeon_crawler_player -1))
    (:`CastFailed`
      (bind _asdungeon_tile_occupant (cast `DungeonTileOccupant` Object))
      (bind _returnvalue (`self.GetType` _asdungeon_tile_occupant))
      (switch `EOccupantType` _returnvalue
        (:`Enemy`
          (`DungeonCrawlerEnemy.AlterHealth` (cast `DungeonCrawlerEnemy` _asdungeon_tile_occupant :!pure true) -1))))))

(fn `UserConstructionScript`
  (bind _tormentor_mesh (`self.Tormentor Mesh`))
  (`PrimitiveComponent.SetMaterial` _tormentor_mesh 1 "/Game/Assets/Materials/MatI_Tormentor.MatI_Tormentor")
  (`MeshComponent.SetScalarParameterValueOnMaterials` _tormentor_mesh "Alpha" 0.0)
  (bind _returnvalue (`AnimSequenceBase.GetPlayLength` (`self.Roar Animation`)))
  (set `self.SpotPlayerActionDuration` _returnvalue))