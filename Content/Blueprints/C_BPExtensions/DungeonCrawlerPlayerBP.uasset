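; Player pawn Blueprint for a tile-based dungeon crawler, handling movement, basic attacks and cooldown-limited dashes between tiles.
; Queued actions spawn highlight previews, then resolve against tile occupants: damaging enemies or a vulnerable Tormentor boss, or collecting eyes, which heal and trigger the exit at six.
; Events update the HUD's health, cooldowns, minimap and proximity tutorial hints.
; Timelines drive material glows for heal and damage.
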(event `self.ReceiveBeginPlay`
  (bind _asplayer_controller (cast `PlayerController` (`self.GetController`)))
  (`KismetSystemLibrary.Delay` 0.2)
  (bind _asgame_hud (cast `/Game/Blueprints/UI/GameHUD` (`PlayerController.GetHUD` _asplayer_controller)))
  (bind _output_get (set `self.HUDRef` _asgame_hud))
  (`/Game/Blueprints/UI/GameHUD.Init HUD` _output_get)
  (`AudioComponent.SetIntParameter` (`self.SC_Hit`) "HitType" 0)
  (`/Game/Blueprints/UI/GameHUD.Display Hint` _output_get "You feel an indescribable sensation compelling you towards the north end of the dungeon." 7.5)
  (bind _asdungeon_gamemode (cast `/Game/Blueprints/DungeonGamemode` (`GameplayStatics.GetGameMode`)))
  (`self.Update Player Minimap Location` _asdungeon_gamemode)
  (`/Game/Blueprints/DungeonGamemode.Track Minimap Update` _asdungeon_gamemode))

(event `self.ReceiveOnAction`
  (params (direction :type "ECardinal Enum" :default "NORTH") (action :type "EPlayerAction Enum" :default "NOACTION") (target :type "DungeonSingleTile Object Reference"))
  (`self.Rotate Player` direction)
  (switch `EPlayerAction` action
    (:`NOACTION`
      (`KismetSystemLibrary.PrintString` "Wuh oh, that's not supposed to happen" false))
    (:`ACTION1`
      (`self.Action - Basic Attack` target))
    (:`ACTION2`
      (`self.Action - Dash` target direction))))

(event `self.ReceiveOnPerform`
  (`self.Adjust CDs`)
  (`/Game/Blueprints/UI/GameHUD.Update Cooldowns` (`self.HUDRef`) (- 1.0 (/ (`KismetMathLibrary.Conv_IntToDouble` (`self.Dash Current CD`)) (`KismetMathLibrary.Conv_IntToDouble` (`self.Dash CD`)))))
  (if (`|EnumEquality` (`self.GetCurrentAction`) "ACTION2")
    (`self.Clear Previews`)
    (`self.Preview - Dash Visual`)))

(event `self.ReceiveOnMove`
  (params (oldPos :type "Vector Structure") (newPos :type "Vector Structure") (newDir :type "ECardinal Enum" :default "NORTH"))
  (`self.Rotate Player` newDir)
  (`self.DispatchMoving`)
  (`KismetSystemLibrary.Delay` (`self.GetActionTime`))
  (`self.DispatchHalt`)
  (bind _asdungeon_gamemode (cast `/Game/Blueprints/DungeonGamemode` (`GameplayStatics.GetGameMode`)))
  (`self.Update Player Minimap Location` _asdungeon_gamemode)
  (if (not (and (`self.Enemy TutATriggered`) (`self.Enemy TutBTriggered`)))
    (`self.ClosestEnemyQuery`)))

(event `self.ReceiveOnDeath`
  (`/Game/Blueprints/UI/GameHUD.DeathEvent` (`self.HUDRef`))
  (`PrimitiveComponent.SetSimulatePhysics` (`self.Player Mesh`) true)
  (`self.EmptyBuffers`)
  (`self.Clear Previews`)
  (`self.DispatchDeath`))

(event `ClosestEnemyQuery`
  (bind _hudref (`self.HUDRef`))
  (bind _returnvalue (`self.GetDistanceTo` (`self.ClosestEnemy`)))
  (bind _returnvalue_2 (`GameplayStatics.GetCurrentLevelName` true))
  (if (`KismetStringLibrary.EqualEqual_StrStr` _returnvalue_2 "DungeonLevel")
    (if (not (and (`self.Enemy TutATriggered`) (`self.Enemy TutBTriggered`)))
      (bind _asdungeon_gamemode (cast `/Game/Blueprints/DungeonGamemode` (`GameplayStatics.GetGameMode`)))
      (bind _activeenemies (`DamnationGameModeBase.ActiveEnemies` _asdungeon_gamemode))
      (bind _output (`|GetArrayItem` _activeenemies))
      (`/Engine/EditorBlueprintResources/StandardMacros.IsValid` _output
        (:`Is Valid`
          (set `self.ClosestEnemy` _output)
          (for (_array_element _array_index) _activeenemies
            (if (!= _array_index 0)
              (if (< (`self.GetSquaredDistanceTo` _array_element) (`self.GetSquaredDistanceTo` (`self.ClosestEnemy`)))
                (set `self.ClosestEnemy` _array_element))))
          (if (<= _returnvalue (`self.EnemyTutADistance`))
            (if (and (> _returnvalue (`self.EnemyTutBDistance`)) (not (`self.Enemy TutATriggered`)))
              (`/Game/Blueprints/UI/GameHUD.Display Hint` _hudref "EnemyTutHint1" 10.0 :!label _label)
              (set `self.Enemy TutATriggered` true)
              (elif (not (`self.Enemy TutATriggered`))
                (goto _label)
                (else
                  (`/Game/Blueprints/UI/GameHUD.Display Hint` _hudref "EnemyTutHint2" 10.0)
                  (set `self.Enemy TutBTriggered` true))))))))
    (else
      (set `self.Enemy TutATriggered` true)
      (set `self.Enemy TutBTriggered` true))))

(event `self.ReceiveOnHealthAltered`
  (params (positiveGain :type Boolean))
  (`/Game/Blueprints/UI/GameHUD.Alter Health` (`self.HUDRef`) (`self.GetHealth`))
  (if (not positiveGain)
    (`self.DispatchHit`)))

(event `self.ReceiveOnActionUpdate`
  (params (action :type "EPlayerAction Enum" :default "NOACTION"))
  (bind _hudref (`self.HUDRef`))
  (`self.Clear Previews`)
  (switch `EPlayerAction` action
    (:`NOACTION`
      (`self.Clear Previews`))
    (:`ACTION1`
      (`/Game/Blueprints/UI/GameHUD.AttackInput` _hudref)
      (`self.Preview - Attack Visual`))
    (:`ACTION2`
      (`/Game/Blueprints/UI/GameHUD.DashInput` _hudref)
      (`self.Preview - Dash Visual`))))

(event `Bind All Eyes Collected To Hint`
  (params (Mural :type "/Game/Blueprints/EyeCheckerBP Object Reference"))
  (add `/Game/Blueprints/EyeCheckerBP.AllEyesCollectedDispatch` Mural (delegate `Display Exit Hint`)))

(event `Display Exit Hint`
  (`/Game/Blueprints/UI/GameHUD.Display Hint` (`self.HUDRef`) "GateOpenHint" 6.5))

(event `Event Lock Player Input`
  (params (Duration :type "Float (double-precision)"))
  (set `self.bLockInput` true)
  (`KismetSystemLibrary.RetriggerableDelay` Duration)
  (set `self.bLockInput` false)
  (`self.DispatchUnlock`)
  (set `self.ActionTime` 0.25))

(event `InputAction|Pause`
  (params (Key :type "Key Structure"))
  (:`Pressed`
    (`/Game/Blueprints/UI/GameHUD.Pause` (`self.HUDRef`))))

(event `PlayerHealAnim`
  (bind _player_mesh (`self.Player Mesh`))
  (`MeshComponent.SetVectorParameterValueOnMaterials` _player_mesh "HighGlowColour" (2.0 10.0 25.0))
  (bind (_direction _alpha) (`Timeline|PlayerHealTimeline` :!via `PlayFromStart`)
    (:`Update`
      (`MeshComponent.SetScalarParameterValueOnMaterials` _player_mesh "Alpha" _alpha))))

(event `InputAction|Display Minimap`
  (params (Key :type "Key Structure"))
  (bind _hudref (`self.HUDRef`))
  (:`Pressed`
    (`/Game/Blueprints/UI/GameHUD.Display Minimap` _hudref))
  (:`Released`
    (`/Game/Blueprints/UI/GameHUD.Hide Minimap` _hudref)))

(event `PlayerDamageAnim`
  (bind _player_mesh (`self.Player Mesh`))
  (`MeshComponent.SetVectorParameterValueOnMaterials` _player_mesh "HighGlowColour" (25.0 10.0 2.0))
  (bind (_direction _alpha) (`Timeline|PlayerDamageTimeline` :!via `PlayFromStart`)
    (:`Update`
      (`MeshComponent.SetScalarParameterValueOnMaterials` _player_mesh "Alpha" _alpha))))

(event `Debug Collect All Eyes`
  (bind _asdungeon_gamemode (cast `/Game/Blueprints/DungeonGamemode` (`GameplayStatics.GetGameMode`)))
  (for _array_element (`DamnationGameModeBase.ActiveEyeTiles` _asdungeon_gamemode)
    (bind _asdungeon_eye_bp (cast `/Game/Blueprints/C_BPExtensions/DungeonEyeBP` (`DungeonSingleTile.OccupyingActor` _array_element)))
    (`/Game/Blueprints/C_BPExtensions/DungeonEyeBP.Collect Eye` _asdungeon_eye_bp)))

(fn `Action - Basic Attack`
  (params (`Target Tile` :type "DungeonSingleTile Object Reference"))
  (bind _asdungeon_tile_occupant (cast `DungeonTileOccupant` (`DungeonSingleTile.OccupyingActor` `Target Tile`))
    (:`then`
      (set `self.Target` _asdungeon_tile_occupant)
      (bind _returnvalue (`DungeonTileOccupant.GetType` _asdungeon_tile_occupant))
      (switch `EOccupantType` _returnvalue
        (:`Boss`
          (bind _asdungeon_tormentor (cast `DungeonTormentor` _asdungeon_tile_occupant :!pure true))
          (bind _asdungeon_tormentor_bp (cast `/Game/Blueprints/C_BPExtensions/DungeonTormentorBP` _asdungeon_tormentor))
          (`/Game/Blueprints/C_BPExtensions/DungeonTormentorBP.TormentorDamageAnim` _asdungeon_tormentor_bp)
          (if (not (`DungeonTormentor.bIsVulnerable` _asdungeon_tormentor))
            (`self.DispatchAttack` false)
            (else
              (`DungeonTormentor.AlterHealth` _asdungeon_tormentor -1)
              (`self.DispatchAttack` true :!label _label))))
        (:`Enemy`
          (`self.Cast And Attack Enemy` _asdungeon_tile_occupant)
          (goto _label))
        (:`Eye`
          (`self.Cast And Collect Eye` _asdungeon_tile_occupant)
          (goto _label))))
    (:`CastFailed`
      (set `self.Target` null)
      (goto _label)))
  (`self.Event Lock Player Input` (+ (`self.GetActionTime`) (`self.Attack Recovery Time`))))

(fn `Action - Dash`
  (params (`Target Tile` :type "DungeonSingleTile Object Reference") (direction :type "ECardinal Enum" :default "NORTH"))
  (locals (Current :type "DungeonSingleTile Object Reference"))
  (bind _returnvalue (+ (`self.GetActionTime`) (`self.Dash Recovery Time`)))
  (if (== (`self.Dash Current CD`) 0)
    (`/Engine/EditorBlueprintResources/StandardMacros.IsValid` `Target Tile` ; Check for early exit if player is dashing into wall/enemy
      (:`Is Valid`
        (bind _output_get (set `local.Current` `Target Tile`))
        (`/Engine/EditorBlueprintResources/StandardMacros.IsValid` (`DungeonSingleTile.OccupyingActor` _output_get)
          (:`Is Valid`
            (`self.Action - Basic Attack` _output_get))
          (:`Is Not Valid`
            (bind _tile (`self.Get Dash Tile` _output_get direction :!label _label))
            (`self.DispatchDash`)
            (set `self.Dash Current CD` (`self.Dash CD`))
            (`/Engine/EditorBlueprintResources/StandardMacros.IsValid` (`DungeonSingleTile.OccupyingActor` _tile)
              (:`Is Valid`
                (`self.Action - Basic Attack` _tile))
              (:`Is Not Valid`
                (`self.JumpToTile` _tile direction)))
            (`self.Event Lock Player Input` _returnvalue)
            (set `self.ActionTime` _returnvalue)
            (`self.DispatchDashRecover`))))
      (:`Is Not Valid`
        (goto _label)))
    (elif (`KismetSystemLibrary.IsValid` (`DungeonSingleTile.OccupyingActor` `Target Tile`))
      (`self.Action - Basic Attack` `Target Tile`)
      (else
        (`self.JumpToTile` `Target Tile` direction)))))

(fn `Action - Swipe Attack`
  (params (`Target Tile` :type "DungeonSingleTile Object Reference") (Direction :type "ECardinal Enum" :default "NORTH"))
  (bind _returnvalue (`DungeonSingleTile.GetAdjacent` `Target Tile` (`DungeonHelpers.RotateCardinal` Direction 1)))
  (bind _returnvalue_2 (`DungeonSingleTile.GetAdjacent` `Target Tile` (`DungeonHelpers.RotateCardinal` Direction -1)))
  (`/Engine/EditorBlueprintResources/StandardMacros.IsValid` `Target Tile`
    (:`Is Valid`
      (`self.Action - Basic Attack` `Target Tile`)
      (`/Engine/EditorBlueprintResources/StandardMacros.IsValid` _returnvalue
        (:`Is Valid`
          (`self.Action - Basic Attack` _returnvalue))
        (:`Is Not Valid`
          _))
      (`/Engine/EditorBlueprintResources/StandardMacros.IsValid` _returnvalue_2
        (:`Is Valid`
          (`self.Action - Basic Attack` _returnvalue_2))))))

(fn `Get Dash Tile`
  (params (`Start Tile` :type "DungeonSingleTile Object Reference") (direction :type "ECardinal Enum" :default "NORTH"))
  (returns (Tile :type "DungeonSingleTile Object Reference"))
  (locals (Current :type "DungeonSingleTile Object Reference"))
  (if (!= (`self.Dash Current CD`) 0)
    (set `local.Current` (`DungeonSingleTile.GetAdjacent` (`self.CurrentTile`) direction))
    (else
      (bind _output_get (set `local.Current` `Start Tile`))
      (for _ (range 1 (+ (`self.Dash Distance`) 1))
        (bind _returnvalue (`DungeonSingleTile.GetAdjacent` _output_get direction))
        (`/Engine/EditorBlueprintResources/StandardMacros.IsValid` _returnvalue
          (:`Is Valid`
            (`/Engine/EditorBlueprintResources/StandardMacros.IsValid` (`DungeonSingleTile.OccupyingActor` _returnvalue)
              (:`Is Valid`
                (return (`local.Current`)))
              (:`Is Not Valid`
                (set `local.Current` _returnvalue))))
          (:`Is Not Valid`
            (break))))))
  (return (`local.Current`)))

(fn `Preview - Dash Visual`
  (bind _enumvalue (foreach `ECardinal` true)
    (:`LoopBody`
      (bind _returnvalue (`DungeonSingleTile.GetConnectedTile` (`self.CurrentTile`) _enumvalue))
      (`/Engine/EditorBlueprintResources/StandardMacros.IsValid` _returnvalue
        (:`Is Valid`
          (bind _tile (`self.Get Dash Tile` _returnvalue _enumvalue))
          (bind _returnvalue_2 (`|SpawnActorFromClass` "/Game/Assets/Prefabs/Fab_PlayerActionHighlight.Fab_PlayerActionHighlight_C" (`self.GetTransform` _tile) "Undefined" "OverrideRootScale" null null))
          (`KismetArrayLibrary.Array_Add` (`self.Active Previews`) _returnvalue_2)
          (`/Game/Assets/Prefabs/Fab_PlayerActionHighlight.Modify Color` _returnvalue_2 (struct :`G` 1.747564 :`B` 4.0 :`A` 1.0))
          (`/Game/Assets/Prefabs/Fab_PlayerActionHighlight.Modify Intensity` _returnvalue_2 0.03 99.0 true)
          (`PrimitiveComponent.SetMaterial` (`/Game/Assets/Prefabs/Fab_PlayerActionHighlight.Bottom` _returnvalue_2) 0 "/Game/Assets/Materials/Decal_DashIndicator.Decal_DashIndicator"))))))

(fn `UserConstructionScript`
  (bind _player_mesh (`self.Player Mesh`))
  (`SceneComponent.K2_AttachToComponent` (`self.Weapon`) (`self.Player Mesh`) "SK_L_HandSocket" "SnapToTarget" "SnapToTarget" "SnapToTarget" true)
  (`PrimitiveComponent.SetMaterial` _player_mesh 0 "/Game/Assets/Materials/MatI_PlayerCharacter.MatI_PlayerCharacter")
  (`PrimitiveComponent.SetMaterial` _player_mesh 1 "/Game/Assets/Materials/MatI_PlayerCharacter.MatI_PlayerCharacter")
  (`MeshComponent.SetScalarParameterValueOnMaterials` _player_mesh "Alpha" 0.0))