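; Room Blueprint, named as a three-way east/south/west variant, that builds its floor when the map loads.
; On OnMapLoad it loops through TileGridFlatArray and, for each valid tile, adds a FloorMesh instance at that tile's world location.
; Each instance gets a random yaw in 90-degree steps, varying the floor through instancing.
; The construction script is empty.
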(event `self.OnMapLoad`
  (for _array_element (`self.TileGridFlatArray`)
    (`/Engine/EditorBlueprintResources/StandardMacros.IsValid` _array_element
      (:`Is Valid`
        (`InstancedStaticMeshComponent.AddInstanceWorldSpace` (`self.FloorMesh`) (`KismetMathLibrary.MakeTransform` (.location (`self.GetTransform` _array_element)) (`KismetMathLibrary.MakeRotator` 0.0 0.0 (* (`KismetMathLibrary.RandomIntegerInRange` 0 3) 90.0))))))))

(fn `UserConstructionScript`)