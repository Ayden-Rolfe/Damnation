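; BossRoomNE is a room Blueprint, named as the north-east boss room, that builds its instanced floor when the map loads.
; OnMapLoad clears FloorMesh, then adds an instance at each valid tile in TileGridFlatArray, yawed in random quarter turns.
; It also copies FloorMeshForced instances overlapping a fixed local box into FloorMesh with the same random rotation, then destroys that placeholder component.
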(event `self.OnMapLoad`
  (bind _floormeshforced (`self.FloorMeshForced`))
  (`InstancedStaticMeshComponent.ClearInstances` (`self.FloorMesh`))
  (for _array_element (`self.TileGridFlatArray`)
    (`/Engine/EditorBlueprintResources/StandardMacros.IsValid` _array_element
      (:`Is Valid`
        (`InstancedStaticMeshComponent.AddInstanceWorldSpace` (`self.FloorMesh`) (`KismetMathLibrary.MakeTransform` (.location (`self.GetTransform` _array_element)) (`KismetMathLibrary.MakeRotator` 0.0 0.0 (* (`KismetMathLibrary.RandomIntegerInRange` 0 3) 90.0)))))))
  (for _array_element_2 (`InstancedStaticMeshComponent.GetInstancesOverlappingBox` _floormeshforced (`KismetMathLibrary.MakeBox` (0.0 0.0 -100.0) (1600.0 1600.0 100.0)) false)
    (`InstancedStaticMeshComponent.AddInstance` (`self.FloorMesh`) (`KismetMathLibrary.MakeTransform` (.location (`InstancedStaticMeshComponent.GetInstanceTransform` _floormeshforced _array_element_2 false)) (`KismetMathLibrary.MakeRotator` 0.0 0.0 (* (`KismetMathLibrary.RandomIntegerInRange` 0 3) 90.0)))))
  (`ActorComponent.K2_DestroyComponent` (`self.FloorMeshForced`)))

(fn `UserConstructionScript`)