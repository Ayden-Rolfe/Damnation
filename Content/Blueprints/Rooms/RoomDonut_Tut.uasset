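; RoomDonut_Tut is a dungeon room Blueprint, apparently a tutorial variant, that builds its floor and shows a boss room hint.
; On map load it rebuilds the instanced FloorMesh from valid TileGridFlatArray actors, giving each tile a random quarter-turn yaw for variety.
; When the player first overlaps PlayerEyeTutTrigger, it displays the "BossRoom" hint through the player's HUD, then destroys the trigger so it fires only once.
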(event `self.OnMapLoad`
  (`InstancedStaticMeshComponent.ClearInstances` (`self.FloorMesh`))
  (for _array_element (`self.TileGridFlatArray`)
    (`/Engine/EditorBlueprintResources/StandardMacros.IsValid` _array_element
      (:`Is Valid`
        (`InstancedStaticMeshComponent.AddInstanceWorldSpace` (`self.FloorMesh`) (`KismetMathLibrary.MakeTransform` (.location (`self.GetTransform` _array_element)) (`KismetMathLibrary.MakeRotator` 0.0 0.0 (* (`KismetMathLibrary.RandomIntegerInRange` 0 3) 90.0))))))))

(event `self.PlayerEyeTutTrigger.OnComponentBeginOverlap`
  (params (OverlappedComponent :type "PrimitiveComponent Object Reference") (OtherActor :type "Actor Object Reference") (OtherComp :type "PrimitiveComponent Object Reference") (OtherBodyIndex :type Integer) (bFromSweep :type Boolean) (SweepResult :type "HitResult Structure (by ref)"))
  (bind _asdungeon_crawler_player_bp (cast `/Game/Blueprints/C_BPExtensions/DungeonCrawlerPlayerBP` OtherActor))
  (`/Game/Blueprints/UI/GameHUD.Display Hint` (`/Game/Blueprints/C_BPExtensions/DungeonCrawlerPlayerBP.HUDRef` _asdungeon_crawler_player_bp) "BossRoom" -1.0)
  (`ActorComponent.K2_DestroyComponent` (`self.PlayerEyeTutTrigger`)))

(fn `UserConstructionScript`)