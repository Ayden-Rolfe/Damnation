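; HallGearNS is a room Blueprint that builds its floor when the map loads.
; On the map-load event it loops over the flat tile grid array and skips invalid entries.
; Each valid tile actor's location receives one instance on the FloorMesh instanced component, yawed randomly in quarter turns to vary the look.
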(event `self.OnMapLoad`
  ;[1 1 1] Floor tile spawn sys- spawns floor tiles
  (for _array_element (`self.TileGridFlatArray`)
    (`/Engine/EditorBlueprintResources/StandardMacros.IsValid` _array_element
      (:`Is Valid`
        (`InstancedStaticMeshComponent.AddInstanceWorldSpace` (`self.FloorMesh`) (`KismetMathLibrary.MakeTransform` (.location (`self.GetTransform` _array_element)) (`KismetMathLibrary.MakeRotator` 0.0 0.0 (* (`KismetMathLibrary.RandomIntegerInRange` 0 3) 90.0))))))))

(fn `UserConstructionScript`)