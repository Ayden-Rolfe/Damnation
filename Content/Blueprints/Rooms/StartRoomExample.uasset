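; Example start room Blueprint that demonstrates hooking custom logic to a map tile event.
; On map load it binds a handler to the tile at a hardcoded grid coordinate and spawns a cone static mesh actor there as a marker.
; When the tile event fires, the handler prints the occupant, the triggered tile and the game time as debug text.
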(event `self.OnMapLoad`
  (bind _returnvalue (`self.GetTile` (`KismetMathLibrary.MakeVector2D` 8.0 6.0)))
  (add `DungeonSingleTile.TileEvent` _returnvalue (delegate `CustomEvent_Wham`))
  (bind _returnvalue_2 (`|SpawnActorFromClass` "/Script/Engine.StaticMeshActor" (`self.GetTransform` _returnvalue) "Undefined" "OverrideRootScale" null null))
  (`StaticMeshComponent.SetStaticMesh` (`StaticMeshActor.StaticMeshComponent` _returnvalue_2) "/Game/StarterContent/Shapes/Shape_Cone.Shape_Cone"))

(event `CustomEvent_Wham`
  (params (Occupant :type "Actor Object Reference") (TriggeredTile :type "DungeonSingleTile Object Reference"))
  (`KismetSystemLibrary.PrintText` (`|FormatText` "Occ. {0} Triggered {1} at {2}!" (`KismetTextLibrary.Conv_StringToText` (`KismetSystemLibrary.GetObjectName` Occupant)) (`KismetTextLibrary.Conv_StringToText` (`KismetSystemLibrary.GetObjectName` TriggeredTile)) (`GameplayStatics.GetTimeSeconds`)) true true (struct :`G` 0.66 :`B` 1.0 :`A` 1.0) 10.0))

(fn `UserConstructionScript`)