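; RoomStart is the dungeon crawler's starting room, building its floor on map load and teaching the player about traps.
; It adds floor instances at each valid grid tile and each forced-floor instance inside the room box, randomly rotated in quarter turns for variety, then destroys the forced-floor component.
; Two trigger volumes show one-time intro and outro trap hints on the player's HUD.
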(event `self.OnMapLoad`
  (bind _floormeshforced (`self.FloorMeshForced`))
  (for _array_element (`self.TileGridFlatArray`)
    (`/Engine/EditorBlueprintResources/StandardMacros.IsValid` _array_element
      (:`Is Valid`
        (`InstancedStaticMeshComponent.AddInstanceWorldSpace` (`self.FloorMesh`) (`KismetMathLibrary.MakeTransform` (.location (`self.GetTransform` _array_element)) (`KismetMathLibrary.MakeRotator` 0.0 0.0 (* (`KismetMathLibrary.RandomIntegerInRange` 0 3) 90.0)))))))
  (for _array_element_2 (`InstancedStaticMeshComponent.GetInstancesOverlappingBox` _floormeshforced (`KismetMathLibrary.MakeBox` (0.0 0.0 -100.0) (1600.0 1600.0 100.0)) false)
    (`InstancedStaticMeshComponent.AddInstance` (`self.FloorMesh`) (`KismetMathLibrary.MakeTransform` (.location (`InstancedStaticMeshComponent.GetInstanceTransform` _floormeshforced _array_element_2 false)) (`KismetMathLibrary.MakeRotator` 0.0 0.0 (* (`KismetMathLibrary.RandomIntegerInRange` 0 3) 90.0)))))
  (`ActorComponent.K2_DestroyComponent` (`self.FloorMeshForced`)))

(event `self.TrapIntroTut.OnComponentBeginOverlap`
  (params (OverlappedComponent :type "PrimitiveComponent Object Reference") (OtherActor :type "Actor Object Reference") (OtherComp :type "PrimitiveComponent Object Reference") (OtherBodyIndex :type Integer) (bFromSweep :type Boolean) (SweepResult :type "HitResult Structure (by ref)"))
  (bind _returnvalue (`GameplayStatics.GetPlayerPawn` 0))
  (if (== OtherActor _returnvalue)
    (if (not (`self.IntroTutTriggered`))
      (bind _asdungeon_crawler_player_bp (cast `/Game/Blueprints/C_BPExtensions/DungeonCrawlerPlayerBP` _returnvalue)
        (:`then`
          (`/Game/Blueprints/UI/GameHUD.Display Hint` (`/Game/Blueprints/C_BPExtensions/DungeonCrawlerPlayerBP.HUDRef` _asdungeon_crawler_player_bp) "TrapTutHint1" -1.0)
          (set `self.IntroTutTriggered` true)
          (`KismetSystemLibrary.PrintString` "IntroTutSuccess" false))
        (:`CastFailed`
          (`KismetSystemLibrary.PrintString` "IntroTutFailure" false :!label _label)))
      (else
        (goto _label)))
    (else
      (goto _label))))

(event `self.TrapOutroTut.OnComponentBeginOverlap`
  (params (OverlappedComponent :type "PrimitiveComponent Object Reference") (OtherActor :type "Actor Object Reference") (OtherComp :type "PrimitiveComponent Object Reference") (OtherBodyIndex :type Integer) (bFromSweep :type Boolean) (SweepResult :type "HitResult Structure (by ref)"))
  (bind _returnvalue (`GameplayStatics.GetPlayerPawn` 0))
  (if (== _returnvalue OtherActor)
    (if (not (`self.OutroTutTriggered`))
      (bind _asdungeon_crawler_player_bp (cast `/Game/Blueprints/C_BPExtensions/DungeonCrawlerPlayerBP` _returnvalue)
        (:`then`
          (bind _hudref (`/Game/Blueprints/C_BPExtensions/DungeonCrawlerPlayerBP.HUDRef` _asdungeon_crawler_player_bp))
          (`/Game/Blueprints/UI/GameHUD.Clear Hint` _hudref)
          (`/Game/Blueprints/UI/GameHUD.Display Hint` _hudref "TrapTutHint2" 10.0)
          (set `self.OutroTutTriggered` true)
          (`KismetSystemLibrary.PrintString` "OutroTutSuccess" false))
        (:`CastFailed`
          (`KismetSystemLibrary.PrintString` "OutroTutFailure" false :!label _label_2)))
      (else
        (goto _label_2)))
    (else
      (goto _label_2))))

(fn `UserConstructionScript`)